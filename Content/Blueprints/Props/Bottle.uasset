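; Bottle prop actor that can be looked at, interacted with and supplied as a throwable mesh.
; Looking at it toggles a custom depth highlight on the mesh; interaction turns off physics and the highlight, and ending it restores physics.
; While IsSpinning is set, Tick rotates the actor around its local pitch axis at a delta-time-scaled rate.
; MeshToThrow exposes the bottle mesh, presumably for the code that throws it.
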(event `self.ReceiveTick`
  (params (DeltaSeconds :type "Float (single-precision)"))
  (`|ExecutionSequence`
    (:`then_1`
      (if (`self.isSpinning`)
        (`self.AddBottleSpin` DeltaSeconds)))))

(event `/Game/Blueprints/Props/Interactible.BeingLookedAt`
  (`PrimitiveComponent.SetRenderCustomDepth` (`self.BottleMesh`) true))

(event `/Game/Blueprints/Props/Interactible.NoLongerLookedAt`
  (`PrimitiveComponent.SetRenderCustomDepth` (`self.BottleMesh`) false))

(event `/Game/Blueprints/Props/Interactible.OnInteractedWith`
  (bind _bottlemesh (`self.BottleMesh`))
  (`PrimitiveComponent.SetSimulatePhysics` _bottlemesh false)
  (`PrimitiveComponent.SetRenderCustomDepth` _bottlemesh false))

(event `/Game/Blueprints/Props/Interactible.OnInteractionEnded`
  (`PrimitiveComponent.SetSimulatePhysics` (`self.BottleMesh`) true))

(fn `AddBottleSpin`
  (params (DeltaTime :type "Float (double-precision)"))
  (`self.K2_AddActorLocalRotation` (`KismetMathLibrary.MakeRotator` 0.0 (* DeltaTime 1000.0))))

(fn `MeshToThrow`
  (returns (mesh :type "StaticMeshComponent Object Reference"))
  (return (`self.BottleMesh`)))

(fn `UserConstructionScript`)